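; MissileDoor is a Blueprint for a door pair that opens through a pressed button, driven by the RaycastPressed input action.
; The press plays a timeline that lerps the button inward and, on each update, plays a second timeline that moves Door and Door1 to the same track-driven relative location.
; Box overlaps enable and disable input on the first-person character itself, and nothing reverses either timeline.
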(event OnComponentBeginOverlap(Box)
  (params (OverlappedComponent :type Primitive%20Component%20Object%20Reference) (OtherActor :type Actor%20Object%20Reference) (OtherComp :type Primitive%20Component%20Object%20Reference) (OtherBodyIndex :type Integer) (bFromSweep :type Boolean) (SweepResult :type Hit%20Result%20Structure%20%28by%20ref%29))
  (bind _asfirst_person_character (Utilities|Casting|CastToFirstPersonCharacter OtherActor))
  (Input|EnableInput _asfirst_person_character (Game|GetPlayerController 0)))

(event OnComponentEndOverlap(Box)
  (params (OverlappedComponent :type Primitive%20Component%20Object%20Reference) (OtherActor :type Actor%20Object%20Reference) (OtherComp :type Primitive%20Component%20Object%20Reference) (OtherBodyIndex :type Integer))
  (bind _asfirst_person_character (Utilities|Casting|CastToFirstPersonCharacter OtherActor))
  (Input|DisableInput _asfirst_person_character (Game|GetPlayerController 0)))

(event Input|ActionEvents|InputActionRaycastPressed
  (params (Key :type Key%20Structure :default "None"))
  (:Pressed
    (Utilities|Casting|CastToFirstPersonCharacter (Game|GetPlayerCharacter 0))
    (bind _buttontrack (Timeline|ButtonPress Play)
      (:Update
        (Transformation|SetRelativeLocation (Variables|Default|GetButton) (Math|Vector|Lerp(Vector) (Variables|Default|GetButton%20Out) (Variables|Default|GetButton%20In) _buttontrack) false false)
        (bind _doortrack (Timeline|Doors Play)
          (:Update
            (Transformation|SetRelativeLocation (Variables|Default|GetDoor1) (Math|Conversions|ToVector(Float) _doortrack) false false)))))))

(fn ConstructionScript)