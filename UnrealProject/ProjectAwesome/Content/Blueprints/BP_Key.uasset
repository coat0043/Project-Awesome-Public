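; BP_Key is a collectible key pickup that adds to the player's key count.
; Its Box overlap enables player input on the actor while the player character is inside and disables it on exit.
; Pressing the RaycastPressed action then increments KeyCount on the FirstPersonCharacter and destroys the key.
; Despite the action's name, pickup relies on proximity, with no trace performed here.
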(event OnComponentBeginOverlap(Box)
  (params (OverlappedComponent :type Primitive%20Component%20Object%20Reference) (OtherActor :type Actor%20Object%20Reference) (OtherComp :type Primitive%20Component%20Object%20Reference) (OtherBodyIndex :type Integer) (bFromSweep :type Boolean) (SweepResult :type Hit%20Result%20Structure%20%28by%20ref%29))
  (if (== OtherActor (Game|GetPlayerCharacter 0))
    (Input|EnableInput (Game|GetPlayerController 0))))

(event OnComponentEndOverlap(Box)
  (params (OverlappedComponent :type Primitive%20Component%20Object%20Reference) (OtherActor :type Actor%20Object%20Reference) (OtherComp :type Primitive%20Component%20Object%20Reference) (OtherBodyIndex :type Integer))
  (if (== (Game|GetPlayerCharacter 0) OtherActor)
    (Input|DisableInput (Game|GetPlayerController 0))))

(event Input|ActionEvents|InputActionRaycastPressed
  (params (Key :type Key%20Structure))
  (:Pressed
    (bind _asfirst_person_character (Utilities|Casting|CastToFirstPersonCharacter (Game|GetPlayerCharacter 0)))
    (bind _result (Math|Integer|IncrementInt (Variables|/Game/FirstPersonCPP/Blueprints/FirstPersonCharacter.FirstPersonCharacter_C|GetKey%20Count _asfirst_person_character))
      (:%20%20
        (Variables|/Game/FirstPersonCPP/Blueprints/FirstPersonCharacter.FirstPersonCharacter_C|SetKey%20Count _asfirst_person_character _result)
        (Actor|DestroyActor)))))

(fn ConstructionScript)